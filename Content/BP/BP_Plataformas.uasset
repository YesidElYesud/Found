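; Platform actor that varies its appearance and acts as a checkpoint for the third-person character.
; The Construction Script gives the cube component a random mesh from an array and a random scale, wide horizontally and thin vertically.
; When the character's capsule overlaps the box trigger, the game instance's SpawnLocation is set slightly above the platform's origin.
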(event OnComponentBeginOverlap(Box)
  (params (OverlappedComponent :type Primitive%20Component%20Object%20Reference) (OtherActor :type Actor%20Object%20Reference) (OtherComp :type Primitive%20Component%20Object%20Reference) (OtherBodyIndex :type Integer) (bFromSweep :type Boolean) (SweepResult :type Hit%20Result%20Structure%20%28by%20ref%29))
  (bind _returnvalue (Transformation|GetActorLocation))
  (bind _asbp_third_person_character (Utilities|Casting|CastToBP_ThirdPersonCharacter OtherActor))
  (if (== OtherComp (Variables|/Script/Engine.Character|GetCapsuleComponent _asbp_third_person_character))
    (bind _asbpgame_instance (Utilities|Casting|CastToBPGameInstance (Game|GetGameInstance)))
    (Variables|/Game/BP/BPGameInstance.BPGameInstance_C|SetSpawn%20Location _asbpgame_instance (Math|Vector|MakeVector (.x _returnvalue) (.y _returnvalue) (+ (.z _returnvalue) 45.0)))))

(event EventBeginPlay)

(event Collision|EventActorBeginOverlap
  (params (OtherActor :type Actor%20Object%20Reference)))

(event EventTick
  (params (DeltaSeconds :type Float%20%28single-precision%29)))

(fn ConstructionScript
  (Components|StaticMesh|SetStaticMesh (Variables|Default|GetCube) (Utilities|Array|Get(acopy) (Variables|Default|GetNew%20Mesh) (Math|Random|RandomIntegerinRange 0 5)))
  (Transformation|SetRelativeScale3D (Variables|Default|GetCube) (Math|Vector|MakeVector (Math|Random|RandomFloatinRange 2.0 3.0) (Math|Random|RandomFloatinRange 2.0 3.0) (Math|Random|RandomFloatinRange 0.1 0.5))))