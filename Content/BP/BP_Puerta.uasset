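; BP_Puerta is a door that breaks away once every campfire in ListaFogatas is lit.
; Each Tick it polls the campfires' EstaEncendido flag, counts the lit ones and raises or lowers the "Cantida" parameter on the Niagara component matched to each index, covering five indices.
; When the count equals the list length it plays an attenuated rock-break sound and destroys itself; otherwise the count resets.
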(event EventBeginPlay)

(event EventTick
  (params (DeltaSeconds :type Float%20%28single-precision%29))
  (bind _listafogatas (Variables|Default|GetListaFogatas))
  (for (_array_element _array_index) _listafogatas
    (if (Variables|/Game/BP/BP_Fogata.BP_Fogata_C|GetEstaEncendido _array_element)
      (Niagara|SetNiagaraVariable(Float) (Utilities|Select :Index _array_index :Option%200 (Variables|Default|GetNiagara4) :Option%201 (Variables|Default|GetNiagara3) :Option%202 (Variables|Default|GetNiagara1) :Option%203 (Variables|Default|GetNiagara) :Option%204 (Variables|Default|GetNiagara2)) "Cantida" 9e+01)
      (Math|Integer|IncrementInt (Variables|Default|GetCON))
      (else
        (Niagara|SetNiagaraVariable(Float) (Utilities|Select :Index _array_index :Option%200 (Variables|Default|GetNiagara4) :Option%201 (Variables|Default|GetNiagara3) :Option%202 (Variables|Default|GetNiagara1) :Option%203 (Variables|Default|GetNiagara) :Option%204 (Variables|Default|GetNiagara2)) "Cantida" 5.0))))
  (if (== (Variables|Default|GetCON) (Utilities|Array|Length _listafogatas))
    (Audio|PlaySoundatLocation "/Game/Sonido/small-rock-break.small-rock-break" (Transformation|GetActorLocation) "0, 0, 0" 1.0 1.0 0.0 "/Game/BP/Enemigos/Fantasma/NewSoundAttenuation.NewSoundAttenuation" 0 0 0)
    (Actor|DestroyActor)
    (else
      (Variables|Default|SetCON 0))))

(fn ConstructionScript)