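; Campfire that lights on first player contact or automatically after a delay, serving as an optional respawn point and ghost repellent.
; Player capsule overlaps can save the spawn location to the game instance and top up the character's Tiempo while below a threshold.
; Ignition timeline grows Niagara fire, point light and repel sphere together; contact ignition also fades a sound parameter.
; Ghosts entering that sphere receive the fire's location and a "Huir" (flee) blackboard flag.
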(event OnComponentBeginOverlap(Sphere2)
  (params (OverlappedComponent :type Primitive%20Component%20Object%20Reference) (OtherActor :type Actor%20Object%20Reference) (OtherComp :type Primitive%20Component%20Object%20Reference) (OtherBodyIndex :type Integer) (bFromSweep :type Boolean) (SweepResult :type Hit%20Result%20Structure%20%28by%20ref%29))
  (bind _asenemy_fantasma (Utilities|Casting|CastToEnemy_Fantasma OtherActor))
  (Variables|/Game/BP/Enemigos/Fantasma/Enemy_Fantasma.Enemy_Fantasma_C|Setdirect _asenemy_fantasma (Transformation|GetActorLocation))
  (AI|Components|Blackboard|SetValueasBool (AI|GetBlackboard (AI|GetAIController _asenemy_fantasma)) (Utilities|Name|MakeLiteralName "Huir") true))

(event OnComponentBeginOverlap(Sphere1)
  (params (OverlappedComponent :type Primitive%20Component%20Object%20Reference) (OtherActor :type Actor%20Object%20Reference) (OtherComp :type Primitive%20Component%20Object%20Reference) (OtherBodyIndex :type Integer) (bFromSweep :type Boolean) (SweepResult :type Hit%20Result%20Structure%20%28by%20ref%29))
  (bind _asbp_third_person_character (Utilities|Casting|CastToBP_ThirdPersonCharacter OtherActor))
  (if (== OtherComp (Variables|/Script/Engine.Character|GetCapsuleComponent _asbp_third_person_character))
    (Variables|Default|SetEstaEncendido true)
    (bind _asbpgame_instance (Utilities|Casting|CastToBPGameInstance (Game|GetGameInstance)))
    (if (Variables|Default|GetGuardaUbi?)
      (Variables|/Game/BP/BPGameInstance.BPGameInstance_C|SetSpawn%20Location _asbpgame_instance (Math|Vector|MakeVector (.x (Transformation|GetActorLocation _asbp_third_person_character)) (.y (Transformation|GetActorLocation _asbp_third_person_character)) (+ (.z (Transformation|GetActorLocation _asbp_third_person_character)) 45.0))))
    (Utilities|FlowControl|Sequence
      (:then_0
        (if (and (Variables|Default|GetPuedeSumarLuz) (> 8e+01 (Variables|/Game/ThirdPerson/Blueprints/BP_ThirdPersonCharacter.BP_ThirdPersonCharacter_C|GetTiempo _asbp_third_person_character)))
          (Variables|/Game/ThirdPerson/Blueprints/BP_ThirdPersonCharacter.BP_ThirdPersonCharacter_C|SetTiempo _asbp_third_person_character (+ (Variables|/Game/ThirdPerson/Blueprints/BP_ThirdPersonCharacter.BP_ThirdPersonCharacter_C|GetTiempo _asbp_third_person_character) (Variables|Default|GetTiempoExtra)))))
      (:then_1
        (Utilities|FlowControl|DoOnce false
          (:Completed
            (CallFunction|Encendido)
            (Components|Activation|Activate (Variables|Default|GetNewNiagaraSystem) true)
            (bind _newtrack_0 (Timeline|Timeline_0 PlayFromStart)
              (:Update
                (Audio|Parameter|SetFloatParameter (Variables|/Script/Engine.AmbientSound|GetAudioComponent (Variables|Default|GetSonidoComp)) (Variables|Default|GetIn%20Name) _newtrack_0 :!class /Script/AudioExtensions.AudioParameterControllerInterface)))))))))

(event Custom|Encendido
  (bind _niagara (Variables|Default|GetNiagara))
  (bind _newtrack_0 (Timeline|Timeline PlayFromStart)
    (:Update
      (Niagara|SetNiagaraVariable(Float) _niagara "Ancho" (Math|Float|MapRangeClamped _newtrack_0 0.0 1.0 1e+01 2e+01))
      (Niagara|SetNiagaraVariable(Float) _niagara "Cantida" (Math|Float|MapRangeClamped _newtrack_0 0.0 1.0 5.0 9e+01))
      (Class|NiagaraComponent|SetNiagaraVariableVec3 _niagara "Escala" (* "1.000000,1.000000,1.000000" (Math|Float|MapRangeClamped _newtrack_0 0.0 1.0 0.1 1.0)))
      (Rendering|Components|Light|SetIntensity (Variables|Default|GetPointLight) (Math|Float|MapRangeClamped _newtrack_0 0.3 1.0 5.0 1.5e+02))
      (Components|Sphere|SetSphereRadius (Variables|Default|GetSphere2) (Math|Float|MapRangeClamped _newtrack_0 0.0 1.0 0.0 3e+02) true))))

(event EventBeginPlay
  (bind _niagara (Variables|Default|GetNiagara))
  (Components|Sphere|SetSphereRadius (Variables|Default|GetSphere2) 0.0 true)
  (Rendering|SetVisibility (Variables|Default|GetSphere) false false)
  (Class|NiagaraComponent|SetNiagaraVariableVec3 _niagara "Escala" "0.100000,0.100000,0.100000")
  (Niagara|SetNiagaraVariable(Float) _niagara "Ancho" 1e+01)
  (Niagara|SetNiagaraVariable(Float) _niagara "Cantida" 5.0)
  (if (Variables|Default|GetAutoEncendido)
    (Utilities|FlowControl|Delay (Variables|Default|GetDely%20AutoEncendido))
    (CallFunction|Encendido)))

(fn ConstructionScript
  (Rendering|Components|Light|SetLightColor (Variables|Default|GetPointLight) (Variables|Default|GetColor%20Luz) true))