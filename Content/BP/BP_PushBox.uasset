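; BP_PushBox is a box the third-person character can push, with a configurable mesh and configurable X and Y movement constraints.
; Overlapping the YBox or XBox trigger enables physics on the mesh and sets the character's EstaEmpujando (pushing) flag; leaving either clears both.
; The construction script assigns the mesh and applies per-axis linear constraint types to a PhysicsConstraint from variables.
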(event OnComponentBeginOverlap(YBox)
  (params (OverlappedComponent :type Primitive%20Component%20Object%20Reference) (OtherActor :type Actor%20Object%20Reference) (OtherComp :type Primitive%20Component%20Object%20Reference) (OtherBodyIndex :type Integer) (bFromSweep :type Boolean) (SweepResult :type Hit%20Result%20Structure%20%28by%20ref%29))
  ;[0.15 0.15 0.15 0.5] Eje Y
  (bind _asbp_third_person_character (Utilities|Casting|CastToBP_ThirdPersonCharacter OtherActor))
  (Physics|SetSimulatePhysics (Variables|Default|GetMalla) true)
  (Variables|/Game/ThirdPerson/Blueprints/BP_ThirdPersonCharacter.BP_ThirdPersonCharacter_C|SetEstaEmpujando? _asbp_third_person_character true))

(event OnComponentEndOverlap(YBox)
  (params (OverlappedComponent :type Primitive%20Component%20Object%20Reference) (OtherActor :type Actor%20Object%20Reference) (OtherComp :type Primitive%20Component%20Object%20Reference) (OtherBodyIndex :type Integer))
  ;[0.15 0.15 0.15 0.5] Eje Y
  (bind _asbp_third_person_character (Utilities|Casting|CastToBP_ThirdPersonCharacter OtherActor))
  (Physics|SetSimulatePhysics (Variables|Default|GetMalla) false)
  (Variables|/Game/ThirdPerson/Blueprints/BP_ThirdPersonCharacter.BP_ThirdPersonCharacter_C|SetEstaEmpujando? _asbp_third_person_character false))

(event OnComponentBeginOverlap(XBox)
  (params (OverlappedComponent :type Primitive%20Component%20Object%20Reference) (OtherActor :type Actor%20Object%20Reference) (OtherComp :type Primitive%20Component%20Object%20Reference) (OtherBodyIndex :type Integer) (bFromSweep :type Boolean) (SweepResult :type Hit%20Result%20Structure%20%28by%20ref%29))
  ;[0.15 0.15 0.15 0.5] Eje X
  (bind _asbp_third_person_character (Utilities|Casting|CastToBP_ThirdPersonCharacter OtherActor))
  (Physics|SetSimulatePhysics (Variables|Default|GetMalla) true)
  (Variables|/Game/ThirdPerson/Blueprints/BP_ThirdPersonCharacter.BP_ThirdPersonCharacter_C|SetEstaEmpujando? _asbp_third_person_character true))

(event OnComponentEndOverlap(XBox)
  (params (OverlappedComponent :type Primitive%20Component%20Object%20Reference) (OtherActor :type Actor%20Object%20Reference) (OtherComp :type Primitive%20Component%20Object%20Reference) (OtherBodyIndex :type Integer))
  ;[0.15 0.15 0.15 0.5] Eje X
  (bind _asbp_third_person_character (Utilities|Casting|CastToBP_ThirdPersonCharacter OtherActor))
  (Physics|SetSimulatePhysics (Variables|Default|GetMalla) false)
  (Variables|/Game/ThirdPerson/Blueprints/BP_ThirdPersonCharacter.BP_ThirdPersonCharacter_C|SetEstaEmpujando? _asbp_third_person_character false))

(fn ConstructionScript
  (bind _physicsconstraint (Variables|Default|GetPhysicsConstraint))
  (Components|StaticMesh|SetStaticMesh (Variables|Default|GetMalla) (Variables|Default|GetMallaRef))
  (Class|PhysicsConstraintComponent|SetLinearXLimit _physicsconstraint (Variables|Default|GetConstraint%20Type%20X) 0.0)
  (Class|PhysicsConstraintComponent|SetLinearYLimit _physicsconstraint (Variables|Default|GetConstraint%20Type%20Y) 0.0))