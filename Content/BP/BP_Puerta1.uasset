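; BP_Puerta1 is a column-mesh door that opens once every campfire in ListaFogatas is lit.
; Tick counts lit fires, and a full count triggers a one-shot sequence.
; With a valid CamRef, the view blends to that camera, the column hides with sound, Niagara and light changes, then returns to the character as the door is destroyed.
; Without one, it plays a positional break sound and destroys itself immediately.
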(event EventBeginPlay
  (Rendering|Components|Light|SetIntensity (Variables|Default|GetPointLight) 0.0))

(event EventTick
  (params (DeltaSeconds :type Float%20%28single-precision%29))
  (bind _listafogatas (Variables|Default|GetListaFogatas))
  (bind _niagara (Variables|Default|GetNiagara))
  (bind _camref (Variables|Default|GetCamRef))
  (for _array_element _listafogatas
    (if (Variables|/Game/BP/BP_FireTotem.BP_FireTotem_C|GetEstaEncendido _array_element)
      (Math|Integer|IncrementInt (Variables|Default|GetCON))))
  (if (== (Variables|Default|GetCON) (Utilities|Array|Length _listafogatas))
    (Utilities|FlowControl|DoOnce false
      (:Completed
        (Utilities|IsValid _camref
          (:Is%20Valid
            (Game|Player|SetViewTargetwithBlend (Game|GetPlayerController 0) _camref 1.0 "VTBlend_EaseInOut" 1.0 false)
            (Utilities|FlowControl|Delay 2.0)
            (Audio|PlaySound2D "/Game/Sonido/small-rock-break.small-rock-break" 1.0 1.0 0.0 0 0)
            (Rendering|SetVisibility (Variables|Default|GetStaticMesh) false false)
            (Niagara|SetNiagaraVariable(Float) _niagara "Ancho" 3e+01)
            (Niagara|SetNiagaraVariable(Float) _niagara "Cantida" 3e+01)
            (Rendering|Components|Light|SetIntensity (Variables|Default|GetPointLight) 6e+01)
            (bind _outactors (Actor|GetAllActorsOfClass "/Game/ThirdPerson/Blueprints/BP_ThirdPersonCharacter.BP_ThirdPersonCharacter_C"))
            (Utilities|FlowControl|Delay 1.0)
            (Game|Player|SetViewTargetwithBlend (Game|GetPlayerController 0) (Utilities|Array|Get(acopy) _outactors) 2.0 "VTBlend_EaseInOut" 2.0 false)
            (Actor|DestroyActor))
          (:Is%20Not%20Valid
            (Audio|PlaySoundatLocation "/Game/Sonido/small-rock-break.small-rock-break" (Transformation|GetActorLocation) "0, 0, 0" 1.0 1.0 0.0 "/Game/BP/Enemigos/Fantasma/NewSoundAttenuation.NewSoundAttenuation" 0 0 0)
            (Actor|DestroyActor)))))
    (else
      (Variables|Default|SetCON 0))))

(fn ConstructionScript
  (Components|StaticMesh|SetStaticMesh (Variables|Default|GetStaticMesh) (Variables|Default|GetColumn)))