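; Torch actor that starts dim and flares up when the player character's capsule enters its box trigger.
; A timeline ramps the Niagara flame's scale and quantity and the point light's intensity, applying ColorLuz as the flame color.
; After a retriggerable delay set by Timer, it jumps back to the BeginPlay dim setup.
; A DoOnce limits ignition to one per overlap, resetting on any end overlap.
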(event OnComponentBeginOverlap(Box)
  (params (OverlappedComponent :type Primitive%20Component%20Object%20Reference) (OtherActor :type Actor%20Object%20Reference) (OtherComp :type Primitive%20Component%20Object%20Reference) (OtherBodyIndex :type Integer) (bFromSweep :type Boolean) (SweepResult :type Hit%20Result%20Structure%20%28by%20ref%29))
  (bind _niagara (Variables|Default|GetNiagara))
  (bind _pointlight (Variables|Default|GetPointLight))
  (bind _asbp_third_person_character (Utilities|Casting|CastToBP_ThirdPersonCharacter OtherActor))
  (if (== (Variables|/Script/Engine.Character|GetCapsuleComponent _asbp_third_person_character) OtherComp)
    (Utilities|FlowControl|DoOnce false
      (:Completed
        (CallFunction|Encendido)
        (Utilities|FlowControl|RetriggerableDelay (Variables|Default|GetTimer))
        (Rendering|Components|Light|SetLightColor _pointlight (Variables|Default|GetColor%20Luz) true)
        (Rendering|Components|Light|SetIntensity _pointlight 1.0)
        (Class|NiagaraComponent|SetNiagaraVariableVec3 _niagara "Escala" "0.100000,0.100000,0.100000")
        (Niagara|SetNiagaraVariable(Float) _niagara "Ancho" 1e+01)
        (Niagara|SetNiagaraVariable(Float) _niagara "Cantida" 5.0)))))

(event OnComponentEndOverlap(Box)
  (params (OverlappedComponent :type Primitive%20Component%20Object%20Reference) (OtherActor :type Actor%20Object%20Reference) (OtherComp :type Primitive%20Component%20Object%20Reference) (OtherBodyIndex :type Integer))
  (bind _niagara (Variables|Default|GetNiagara))
  (bind _pointlight (Variables|Default|GetPointLight))
  (Utilities|FlowControl|DoOnce false) ; enters at Reset
)

(event Custom|Encendido
  (bind _niagara (Variables|Default|GetNiagara))
  (bind _newtrack_0 (Timeline|Timeline PlayFromStart)
    (:Update
      (Niagara|SetNiagaraVariable(Float) _niagara "Ancho" (Math|Float|MapRangeClamped _newtrack_0 0.0 1.0 1e+01 1e+01))
      (Niagara|SetNiagaraVariable(Float) _niagara "Cantida" (Math|Float|MapRangeClamped _newtrack_0 0.0 1.0 5.0 2e+01))
      (Class|NiagaraComponent|SetNiagaraVariableVec3 _niagara "Escala" (* "1.000000,1.000000,1.000000" (Math|Float|MapRangeClamped _newtrack_0 0.0 1.0 0.1 0.5)))
      (Niagara|SetNiagaraVariable(LinearColor) _niagara "FlameColor" (Variables|Default|GetColor%20Luz))
      (Rendering|Components|Light|SetIntensity (Variables|Default|GetPointLight) (Math|Float|MapRangeClamped _newtrack_0 0.3 1.0 5.0 1.5e+02)))))

(event EventBeginPlay
  (bind _niagara (Variables|Default|GetNiagara))
  (bind _pointlight (Variables|Default|GetPointLight))
  (Rendering|Components|Light|SetLightColor _pointlight (Variables|Default|GetColor%20Luz) true)
  (Rendering|Components|Light|SetIntensity _pointlight 1.0)
  (Class|NiagaraComponent|SetNiagaraVariableVec3 _niagara "Escala" "0.100000,0.100000,0.100000")
  (Niagara|SetNiagaraVariable(Float) _niagara "Ancho" 1e+01)
  (Niagara|SetNiagaraVariable(Float) _niagara "Cantida" 5.0))

(fn ConstructionScript)